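; BP_Cube is a physics cube that the player can levitate, attract and propel.
; OnInteract toggles levitation: it disables gravity, drives the mesh's relative Z from a timeline and applies a translucent material, or restores gravity and material.
; Attract moves the mesh to the player pawn's location and zeroes velocity on completion, while Stop interrupts that move.
; Propulse applies a mass-independent impulse and ends levitation, restoring gravity and material.
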(event `self.ReceiveBeginPlay`
  (bind _returnvalue (`self.GetComponentByClass` "/Script/Engine.StaticMeshComponent"))
  (`KismetSystemLibrary.PrintString` (`KismetSystemLibrary.GetDisplayName` _returnvalue))
  (bind _output_get (set `self.Usable Mesh` _returnvalue))
  (`KismetSystemLibrary.PrintString` (`KismetSystemLibrary.GetDisplayName` _output_get))
  (set `self.BaseMaterial` (`PrimitiveComponent.GetMaterial` (`self.Usable Mesh`) 0)))

(event `self.OnInteract`
  (params (InteractingPlayer :type "Character Object Reference"))
  (bind _usable_mesh (`self.Usable Mesh`))
  (bind _usable_mesh_2 (`self.Usable Mesh`))
  (bind (_relativelocation_x _relativelocation_y) (`KismetMathLibrary.BreakVector` (`SceneComponent.RelativeLocation` _usable_mesh_2)))
  (if (`self.IsLevitating_0`)
    (`KismetSystemLibrary.PrintString` "oulala je vole plus")
    (set `self.IsLevitating_0` false)
    (`self.Levitate?`)
    (`PrimitiveComponent.SetEnableGravity` _usable_mesh true)
    (`PrimitiveComponent.SetMaterial` (`self.Usable Mesh`) 0 (`self.BaseMaterial`))
    (else
      (`KismetSystemLibrary.PrintString` "oulala je vole")
      (set `self.IsLevitating_0` true)
      (`self.Levitate?`)
      (`PrimitiveComponent.SetEnableGravity` _usable_mesh false)
      (bind (_direction _float) (`Timeline|StartLevitate` :!via `PlayFromStart`)
        (:`Update`
          (`SceneComponent.K2_SetRelativeLocation` _usable_mesh_2 (`KismetMathLibrary.MakeVector` _relativelocation_x _relativelocation_y _float) false false)
          (`PrimitiveComponent.SetMaterial` (`self.Usable Mesh`) 0 "/Game/Material/M_Translucent.M_Translucent"))))))

(event `self.Attract`
  (params (IsComing :type "Character Object Reference"))
  (bind _usable_mesh (`self.Usable Mesh`))
  (`KismetSystemLibrary.MoveComponentTo` _usable_mesh (`self.K2_GetActorLocation` (`GameplayStatics.GetPlayerPawn` 0)) (struct) false false 1.0 :!label _label)
  (`PrimitiveComponent.SetPhysicsLinearVelocity` _usable_mesh (0.0 0.0 0.0) false "None"))

(event `self.Stop`
  (params (InteractingPlayer :type "Character Object Reference"))
  (goto _label :!via `Stop`))

(event `self.Propulse`
  (params (PropulseLocation :type "Vector Structure"))
  (bind _usable_mesh (`self.Usable Mesh`))
  (`PrimitiveComponent.AddImpulse` _usable_mesh PropulseLocation "None" true)
  (`PrimitiveComponent.SetEnableGravity` _usable_mesh true)
  (set `self.IsLevitating_0` false)
  (`PrimitiveComponent.SetMaterial` (`self.Usable Mesh`) 0 (`self.BaseMaterial`)))

(fn `IsInteractable`
  (returns (Interactable :type Boolean))
  (return false))

(fn `Levitate?`
  (returns (`Levitating?` :type Boolean))
  (if (`self.IsLevitating_0`)
    (return true)
    (else
      (return false))))

(fn `UserConstructionScript`)